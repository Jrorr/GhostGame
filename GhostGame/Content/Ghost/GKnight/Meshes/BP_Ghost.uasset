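; Ghost knight AI enemy that patrols the house invisibly, then haunts the player once no Artifact actors remain.
; Patrol chains AI moves through five preset points, using flags to resume the current leg.
; While invisible, sighting a pawn runs the artifact check, which reveals the ghost through material swaps and ends patrol.
; Tick then drives constant pursuit of the player, and sighting Bryson while visible also triggers the ghost sound.
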(event `self.ReceiveBeginPlay`
  (bind _output_get (set `self.Visible` false))
  (`self.Change visibilty` _output_get)
  (set `self.Patroling` true)
  (`self.Patrol`)
  (bind _returnvalue (`AddComponent|NODE_AddAudioComponent-1`))
  (`AudioComponent.Stop` _returnvalue)
  (set `self.GhostSound` _returnvalue))

(event `HauntPlayer`
  (bind _outactors (`GameplayStatics.GetAllActorsOfClass` "/Game/HauntManager/Artifact.Artifact_C"))
  (if (<= (`KismetArrayLibrary.Array_Length` _outactors) 0)
    (bind _output_get (set `self.Visible` true))
    (`self.Change visibilty` _output_get)
    (set `self.Patroling` false)))

(event `self.PawnSensing.OnSeePawn`
  (params (Pawn :type "Pawn Object Reference"))
  ;[1 1 1] Chase mode: If the ghost sees the player, it will play ghost sound and chase them.
  (if (`self.Visible`)
    (bind _asbryson_character (cast `/Game/ThirdPersonBP/Blueprints/Bryson_Character` Pawn))
    (`|ExecutionSequence`
      (:`then_0`
        (set `self.CanSeeEnemy?` true)
        (`|AIMoveTo` self (0.0 0.0 0.0) _asbryson_character
          (:`then`
            (`/Engine/EditorBlueprintResources/StandardMacros.DoOnce` false :!label _label
              (:`Completed`
                (`AudioComponent.Play` (`self.GhostSound`) 0.0))))))
      (:`then_1`
        (`KismetSystemLibrary.RetriggerableDelay` 0.6)
        (set `self.CanSeeEnemy?` false)))
    (elif (`self.Patroling`)
      (`self.HauntPlayer`))))

(event `self.ReceiveTick`
  (params (DeltaSeconds :type "Float (single-precision)"))
  ;[1 1 1] Chase mode: If the ghost sees the player, it will play ghost sound and chase them.
  (if (`self.Patroling`)
    (if (not (`self.CanSeeEnemy?`))
      (`KismetSystemLibrary.Delay` 0.4)
      (if (not (`self.CanSeeEnemy?`))
        (`AudioComponent.FadeOut` (`self.GhostSound`) 2.0 0.0 "Linear")
        (`self.Patrol`)
        (goto _label :!via `Reset`)))
    (else
      (`|AIMoveTo` self (0.0 0.0 0.0) (`GameplayStatics.GetPlayerPawn` 0)))))

(event `Patrol`
  ;[1 1 1] Patrol: Move around the house to preset positions
  (if (`self.Patroling`)
    (if (`self.Patrol Location 1`)
      (`|AIMoveTo` self (+ (`self.Patrol Vector 1`) (`KismetMathLibrary.MakeVector` (`KismetMathLibrary.RandomFloatInRange` 0.0 200.0) 0.0 (`KismetMathLibrary.RandomFloatInRange` 0.0 200.0))) null
        (:`OnSuccess`
          (`self.Patrol Locations` false true :!label _label_2
            (:`Out`
              (`|AIMoveTo` self (`self.Patrol Vector 2`) null
                (:`OnSuccess`
                  (`self.Patrol Locations` false false true :!label _label_3
                    (:`Out`
                      (`|AIMoveTo` self (`self.Patrol Vector 3`) null
                        (:`OnSuccess`
                          (`self.Patrol Locations` false false false true :!label _label_4
                            (:`Out`
                              (`|AIMoveTo` self (`self.Patrol Vector 4`) null
                                (:`OnSuccess`
                                  (`self.Patrol Locations` false false false false true :!label _label_5
                                    (:`Out`
                                      (`|AIMoveTo` self (`self.Patrol Vector 5`) null
                                        (:`OnSuccess`
                                          (`self.Patrol Locations` true false false false true
                                            (:`Out`
                                              (`self.Patrol`)))))))))))))))))))))
      (elif (`self.Patrol Location 2`)
        (goto _label_2)
        (elif (`self.Patrol Location  3`)
          (goto _label_3)
          (elif (`self.Patrol Location  4`)
            (goto _label_4)
            (elif (`self.Patrol Location  5`)
              (goto _label_5))))))))

(fn `Change visibilty`
  (params (Visibility :type Boolean))
  (if Visibility
    (for (_array_element _array_index) (`self.Materials`)
      (`PrimitiveComponent.SetMaterial` (`self.Mesh`) _array_index _array_element))
    (else
      (for (_ _array_index_2) (`MeshComponent.GetMaterials` (`self.Mesh`))
        (if (== _array_index_2 4)
          (`PrimitiveComponent.SetMaterial` (`self.Mesh`) _array_index_2 "/Game/Ghost/GKnight/Materials/MI_GKnightSkirt_hide.MI_GKnightSkirt_hide" :!label _label)
          (elif (== _array_index_2 5)
            (goto _label)
            (else
              (`PrimitiveComponent.SetMaterial` (`self.Mesh`) _array_index_2 "/Game/Ghost/GKnight/Materials/Invis_Inst.Invis_Inst"))))))))

(fn `UserConstructionScript`)